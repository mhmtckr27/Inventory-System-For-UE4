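; BP_Inventory is the Blueprint layer of the inventory system, connecting inherited inventory logic to its on-screen UI.
; CreateWidgets builds the main widget with itself as the inventory, caches the nested inventory widget, initializes the weight display and adds it to the viewport.
; Slot and weight events refresh the matching widgets.
; AddItem wraps the parent implementation, queuing a collected-item notification for the amount actually added on success.
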(event EventOnWeightChanged
  (Default|UpdateWeight (Variables|Default|GetWBP_InventoryWidget) (Variables|Default|GetCurrentCarryWeight) (Variables|Default|GetMaxCarryWeight)))

(event EventOnUpdateSlotatIndex
  (params (SlotIndex :type Integer))
  (Default|OnUpdateSlot (Utilities|Array|Get(acopy) (Variables|/Game/InventorySystemCPP/Blueprints/Widgets/WBP_Inventory.WBP_Inventory_C|GetSlotWidgets (Variables|Default|GetWBP_InventoryWidget)) SlotIndex)))

(fn ConstructionScript)

(fn CreateWidgets
  (bind _returnvalue (UserInterface|CreateWidget "/Game/InventorySystemCPP/Blueprints/Widgets/WBP_Main.WBP_Main_C" 0 self (Variables|Default|GetColumnCount) (Variables|Default|GetCollected%20Item%20Notification%20Stay%20Duration)))
  (bind _output_get (Variables|Default|SetWBP_MainWidget _returnvalue))
  (Variables|Default|SetWBP_InventoryWidget (Variables|/Game/InventorySystemCPP/Blueprints/Widgets/WBP_Main.WBP_Main_C|GetWBP_Inventory _output_get))
  (Default|UpdateWeight (Variables|/Game/InventorySystemCPP/Blueprints/Widgets/WBP_Main.WBP_Main_C|GetWBP_Inventory _output_get) (Variables|Default|GetCurrentCarryWeight) (Variables|Default|GetMaxCarryWeight))
  (UserInterface|Viewport|AddtoViewport (Variables|Default|GetWBP_MainWidget) 0))

(fn AddItem
  (params (ItemClass :type Item%20Base%20Class%20Reference) (AmountToAdd :type Integer))
  (bind (_remainingamount _returnvalue) (|CallParentFunction ItemClass AmountToAdd))
  (if _returnvalue
    (Default|AddtoCollectedItemQueue (Variables|Default|GetWBP_MainWidget) ItemClass (- AmountToAdd _remainingamount))
    (return _remainingamount _returnvalue)
    (else
      (return _remainingamount _returnvalue))))