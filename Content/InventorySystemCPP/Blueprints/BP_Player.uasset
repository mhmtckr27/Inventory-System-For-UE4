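; Player Blueprint that gives the player an inventory and a key to show or hide its UI.
; On BeginPlay it spawns a BP_Inventory actor with itself as Player, stores it in both Inventory and BPInventory, and has it create its widgets.
; Pressing I toggles the visibility of the inventory widget held by that actor.
; The construction script only calls its parent.
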(event EventBeginPlay
  (bind _returnvalue (Game|SpawnActorfromClass "/Game/InventorySystemCPP/Blueprints/BP_Inventory.BP_Inventory_C" (Math|Transform|MakeTransform "0, 0, 0" "0, 0, 0" "1,1,1") "Undefined" 0 self 4 0))
  (Variables|Default|SetInventory _returnvalue)
  (bind _output_get (Variables|Default|SetBP_Inventory _returnvalue))
  (Default|CreateWidgets _output_get))

(event Input|KeyboardEvents|I
  (params (Key :type Key%20Structure :default "None"))
  (:Pressed
    (Default|ToggleVisibility (Variables|/Game/InventorySystemCPP/Blueprints/BP_Inventory.BP_Inventory_C|GetWBP_InventoryWidget (Variables|Default|GetBP_Inventory)))))

(fn ConstructionScript
  (|CallParentFunction))